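; Modular fantasy sword actor that assembles a grip, crossguard, blade and pommel from selectable skeletal meshes in its Construction Script.
; Crossguard and pommel snap to grip sockets and the blade to the crossguard's, with adjustable blade and pommel scale and optional per-blade animation.
; Each part gets a dynamic material for layered surface settings, plus blade emissive and shared dirt, damage and blood.
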(fn `UserConstructionScript`
  (bind _crossguardmesh (`self.CrossguardMesh`))
  (bind _blademesh (`self.BladeMesh`))
  (bind _pommelmesh (`self.PommelMesh`))
  (bind _gripmesh (`self.GripMesh`))
  (bind _output (`|GetArrayItem` (`self.Blades`) (`self.Blade`)))
  (`|ExecutionSequence`
    (:`then_0`
      ;[1 1 1] Grip_Mesh
      (`SkinnedMeshComponent.SetSkinnedAssetAndUpdate` (`self.GripMesh`) (`|GetArrayItem` (`self.Grips`) (`self.Grip`)) true)
      (bind _returnvalue (`PrimitiveComponent.CreateDynamicMaterialInstance` _gripmesh 0 (`PrimitiveComponent.GetMaterial` _gripmesh 0) "None"))
      (bind _output_get (set `self.Material Grip` _returnvalue))
      (`PrimitiveComponent.SetMaterial` (`self.GripMesh`) 0 _output_get)
      (`|ExecutionSequence`
        (:`then_0`
          ;[1 1 1] Sword Material 1
          (bind _output_get_2 (set `self.Material1Values` (`|MakeMap` "M1_Metalness" (`self.Grip M1 - Metallic`) "M1_Roughness_Overlay" (`self.Grip M1 - RoughnessOverlay`) "M1_Normal_Multiply" (`self.Grip M1 - Normal Multiply`) "M1_Texture_Rotator" (`self.Grip M1 - Texture Rotation`) "M1_Texture_Tilling" (`self.Grip M1 - Texture Tiling`))))
          (bind _keys (`BlueprintMapLibrary.Map_Keys` _output_get_2))
          (for _array_element _keys
            (`MaterialInstanceDynamic.SetScalarParameterValue` (`self.Material Grip`) (`KismetStringLibrary.Conv_StringToName` _array_element) (`BlueprintMapLibrary.Map_Find` (`self.Material1Values`) _array_element)))
          (`MaterialInstanceDynamic.SetTextureParameterValue` (`self.Material Grip`) "M1_Normal" (`self.Grip M1 - Normal Map`))
          (`MaterialInstanceDynamic.SetTextureParameterValue` (`self.Material Grip`) "M1_Texture" (`self.Grip M1 - Texture`))
          (`MaterialInstanceDynamic.SetVectorParameterValue` (`self.Material Grip`) "M1_Material_Color" (`self.Grip M1 - Material Color`)))
        (:`then_1`
          ;[1 1 1] Sword Material 2
          (bind _output_get_3 (set `self.Material2Values` (`|MakeMap` "M2_Metalness" (`self.Grip M2 - Metallic`) "M2_Roughness_Overlay" (`self.Grip M2 - RoughnessOverlay`) "M2_Normal_Multiply" (`self.Grip M2 - Normal Multiply`) "M2_Texture_Rotator" (`self.Grip M2 - Texture Rotation`) "M2_Texture_Tilling" (`self.Grip M2 - Texture Tiling`))))
          (bind _keys_2 (`BlueprintMapLibrary.Map_Keys` _output_get_3))
          (for _array_element_2 _keys_2
            (`MaterialInstanceDynamic.SetScalarParameterValue` (`self.Material Grip`) (`KismetStringLibrary.Conv_StringToName` _array_element_2) (`BlueprintMapLibrary.Map_Find` (`self.Material2Values`) _array_element_2)))
          (`MaterialInstanceDynamic.SetTextureParameterValue` (`self.Material Grip`) "M2_Normal" (`self.Grip M2 - Normal Map`))
          (`MaterialInstanceDynamic.SetTextureParameterValue` (`self.Material Grip`) "M2_Texture" (`self.Grip M2 - Texture`))
          (`MaterialInstanceDynamic.SetVectorParameterValue` (`self.Material Grip`) "M2_Material_Color" (`self.Grip M2 - Material Color`)))
        (:`then_2`
          ;[1 1 1] Sword Material 3
          (bind _output_get_4 (set `self.Material3Values` (`|MakeMap` "M3_Metalness" (`self.Grip M3 - Metallic`) "M3_Roughness_Overlay" (`self.Grip M3 - RoughnessOverlay`) "M3_Normal_Multiply" (`self.Grip M3 - Normal Multiply`) "M3_Texture_Rotator" (`self.Grip M3 - Texture Rotation`) "M3_Texture_Tilling" (`self.Grip M3 - Texture Tiling`))))
          (bind _keys_3 (`BlueprintMapLibrary.Map_Keys` _output_get_4))
          (for _array_element_3 _keys_3
            (`MaterialInstanceDynamic.SetScalarParameterValue` (`self.Material Grip`) (`KismetStringLibrary.Conv_StringToName` _array_element_3) (`BlueprintMapLibrary.Map_Find` (`self.Material3Values`) _array_element_3)))
          (`MaterialInstanceDynamic.SetTextureParameterValue` (`self.Material Grip`) "M3_Normal" (`self.Grip M3 - Normal Map`))
          (`MaterialInstanceDynamic.SetTextureParameterValue` (`self.Material Grip`) "M3_Texture" (`self.Grip M3 - Texture`))
          (`MaterialInstanceDynamic.SetVectorParameterValue` (`self.Material Grip`) "M3_Material_Color" (`self.Grip M3 - Material Color`)))))
    (:`then_1`
      ;[1 1 1] Crossguard_Mesh
      (`SkinnedMeshComponent.SetSkinnedAssetAndUpdate` (`self.CrossguardMesh`) (`|GetArrayItem` (`self.Crossguards`) (`self.Crossguard`)) true)
      (`SceneComponent.K2_SetRelativeTransform` (`self.CrossguardMesh`) (`SceneComponent.GetSocketTransform` (`self.GripMesh`) "CrossGuard" "RTS_Actor") false false)
      (bind _returnvalue_2 (`PrimitiveComponent.CreateDynamicMaterialInstance` _crossguardmesh 0 (`PrimitiveComponent.GetMaterial` _crossguardmesh 0) "None"))
      (bind _output_get_5 (set `self.Material Crossguard` _returnvalue_2))
      (`PrimitiveComponent.SetMaterial` (`self.CrossguardMesh`) 0 _output_get_5)
      ;[1 1 1] Cross-guard Material 1
      (bind _output_get_6 (set `self.Material1Values` (`|MakeMap` "M1_Metalness" (`self.Cross M1 - Metallic`) "M1_Roughness_Overlay" (`self.Cross M1 - RoughnessOverlay`) "M1_Normal_Multiply" (`self.Cross M1 - Normal Multiply`) "M1_Texture_Rotator" (`self.Cross M1 - Texture Rotation`) "M1_Texture_Tilling" (`self.Cross M1 - Texture Tiling`))))
      (bind _keys_4 (`BlueprintMapLibrary.Map_Keys` _output_get_6))
      (for _array_element_4 _keys_4
        (`MaterialInstanceDynamic.SetScalarParameterValue` (`self.Material Crossguard`) (`KismetStringLibrary.Conv_StringToName` _array_element_4) (`BlueprintMapLibrary.Map_Find` (`self.Material1Values`) _array_element_4)))
      (`MaterialInstanceDynamic.SetTextureParameterValue` (`self.Material Crossguard`) "M1_Normal" (`self.Cross M1 - Normal Map`))
      (`MaterialInstanceDynamic.SetTextureParameterValue` (`self.Material Crossguard`) "M1_Texture" (`self.Cross M1 - Texture`))
      (`MaterialInstanceDynamic.SetVectorParameterValue` (`self.Material Crossguard`) "M1_Material_Color" (`self.Cross M1 - Material Color`)))
    (:`then_2`
      ;[1 1 1] Blade_Mesh
      (`SkinnedMeshComponent.SetSkinnedAssetAndUpdate` (`self.BladeMesh`) _output true)
      (`SceneComponent.K2_SetRelativeTransform` (`self.BladeMesh`) (`SceneComponent.GetSocketTransform` (`self.CrossguardMesh`) "Blade" "RTS_Actor") false false)
      (`SceneComponent.SetRelativeScale3D` (`self.BladeMesh`) (`self.Blade Scale`))
      (bind _returnvalue_3 (`PrimitiveComponent.CreateDynamicMaterialInstance` _blademesh 0 (`PrimitiveComponent.GetMaterial` _blademesh 0) "None"))
      (bind _output_get_7 (set `self.Material Blade` _returnvalue_3))
      (`PrimitiveComponent.SetMaterial` (`self.BladeMesh`) 0 _output_get_7)
      (bind _output_get_8 (set `self.Blade Animation` (`BlueprintMapLibrary.Map_Find` (`self.BladeAnimations`) _output)))
      (`/Engine/EditorBlueprintResources/StandardMacros.IsValid` _output_get_8
        (:`Is Valid`
          (`SkeletalMeshComponent.OverrideAnimationData` (`self.BladeMesh`) (`self.Blade Animation`) true true 0.0 1.0))
        (:`Is Not Valid`
          _))
      (`|ExecutionSequence`
        (:`then_0`
          ;[1 1 1] Sword Material 1
          (bind _output_get_9 (set `self.Material1Values` (`|MakeMap` "M1_Metalness" (`self.Blade M1 - Metallic`) "M1_Roughness_Overlay" (`self.Blade M1 - RoughnessOverlay`) "M1_Normal_Multiply" (`self.Blade M1 - Normal Multiply`) "M1_Texture_Rotator" (`self.Blade M1 - Texture Rotation`) "M1_Texture_Tilling" (`self.Blade M1 - Texture Tiling`))))
          (bind _keys_5 (`BlueprintMapLibrary.Map_Keys` _output_get_9))
          (for _array_element_5 _keys_5
            (`MaterialInstanceDynamic.SetScalarParameterValue` (`self.Material Blade`) (`KismetStringLibrary.Conv_StringToName` _array_element_5) (`BlueprintMapLibrary.Map_Find` (`self.Material1Values`) _array_element_5)))
          (`MaterialInstanceDynamic.SetTextureParameterValue` (`self.Material Blade`) "M1_Normal" (`self.Blade M1 - Normal Map`))
          (`MaterialInstanceDynamic.SetTextureParameterValue` (`self.Material Blade`) "M1_Texture" (`self.Blade M1 - Texture`))
          (`MaterialInstanceDynamic.SetVectorParameterValue` (`self.Material Blade`) "M1_Material_Color" (`self.Blade M1 - Material Color`)))
        (:`then_1`
          ;[1 1 1] Sword Material 2
          (bind _output_get_10 (set `self.Material2Values` (`|MakeMap` "M2_Metalness" (`self.Blade M2 - Metallic`) "M2_Roughness_Overlay" (`self.Blade M2 - RoughnessOverlay`) "M2_Normal_Multiply" (`self.Blade M2 - Normal Multiply`) "M2_Texture_Rotator" (`self.Blade M2 - Texture Rotation`) "M2_Texture_Tilling" (`self.Blade M2 - Texture Tiling`))))
          (bind _keys_6 (`BlueprintMapLibrary.Map_Keys` _output_get_10))
          (for _array_element_6 _keys_6
            (`MaterialInstanceDynamic.SetScalarParameterValue` (`self.Material Blade`) (`KismetStringLibrary.Conv_StringToName` _array_element_6) (`BlueprintMapLibrary.Map_Find` (`self.Material2Values`) _array_element_6)))
          (`MaterialInstanceDynamic.SetTextureParameterValue` (`self.Material Blade`) "M2_Normal" (`self.Blade M2 - Normal Map`))
          (`MaterialInstanceDynamic.SetTextureParameterValue` (`self.Material Blade`) "M2_Texture" (`self.Blade M2 - Texture`))
          (`MaterialInstanceDynamic.SetVectorParameterValue` (`self.Material Blade`) "M2_Material_Color" (`self.Blade M2 - Material Color`)))
        (:`then_2`
          ;[1 1 1] Sword Material 3
          (bind _output_get_11 (set `self.Material3Values` (`|MakeMap` "M3_Metalness" (`self.Blade M3 - Metallic`) "M3_Roughness_Overlay" (`self.Blade M3 - RoughnessOverlay`) "M3_Normal_Multiply" (`self.Blade M3 - Normal Multiply`) "M3_Texture_Rotator" (`self.Blade M3 - Texture Rotation`) "M3_Texture_Tilling" (`self.Blade M3 - Texture Tiling`))))
          (bind _keys_7 (`BlueprintMapLibrary.Map_Keys` _output_get_11))
          (for _array_element_7 _keys_7
            (`MaterialInstanceDynamic.SetScalarParameterValue` (`self.Material Blade`) (`KismetStringLibrary.Conv_StringToName` _array_element_7) (`BlueprintMapLibrary.Map_Find` (`self.Material3Values`) _array_element_7)))
          (`MaterialInstanceDynamic.SetTextureParameterValue` (`self.Material Blade`) "M3_Normal" (`self.Blade M3 - Normal Map`))
          (`MaterialInstanceDynamic.SetTextureParameterValue` (`self.Material Blade`) "M3_Texture" (`self.Blade M3 - Texture`))
          (`MaterialInstanceDynamic.SetVectorParameterValue` (`self.Material Blade`) "M3_Material_Color" (`self.Blade M3 - Material Color`)))
        (:`then_3`
          ;[1 1 1] Emissive
          (`MaterialInstanceDynamic.SetVectorParameterValue` (`self.Material Blade`) "Emissive_Color_1" (`self.Emissive Material Color`))
          (`MaterialInstanceDynamic.SetScalarParameterValue` (`self.Material Blade`) "Emissive_Multiply" (`self.Emissive Multiply`)))))
    (:`then_3`
      ;[1 1 1] Pommel_Mesh
      (`SkinnedMeshComponent.SetSkinnedAssetAndUpdate` (`self.PommelMesh`) (`|GetArrayItem` (`self.Pommels`) (`self.Pommel`)) true)
      (`SceneComponent.K2_SetRelativeTransform` (`self.PommelMesh`) (`SceneComponent.GetSocketTransform` (`self.GripMesh`) "Pommel" "RTS_Actor") false false)
      (`SceneComponent.SetRelativeScale3D` (`self.PommelMesh`) (`self.Pommel Scale`))
      (bind _returnvalue_4 (`PrimitiveComponent.CreateDynamicMaterialInstance` _pommelmesh 0 (`PrimitiveComponent.GetMaterial` _pommelmesh 0) "None"))
      (bind _output_get_12 (set `self.Material Pommel` _returnvalue_4))
      (`PrimitiveComponent.SetMaterial` (`self.PommelMesh`) 0 _output_get_12)
      ;[1 1 1] Pommel Material 1
      (bind _output_get_13 (set `self.Material1Values` (`|MakeMap` "M1_Metalness" (`self.Pommel M1 - Metallic`) "M1_Roughness_Overlay" (`self.Pommel M1 - RoughnessOverlay`) "M1_Normal_Multiply" (`self.Pommel M1 - Normal Multiply`) "M1_Texture_Rotator" (`self.Pommel M1 - Texture Rotation`) "M1_Texture_Tilling" (`self.Pommel M1 - Texture Tiling`))))
      (bind _keys_8 (`BlueprintMapLibrary.Map_Keys` _output_get_13))
      (for _array_element_8 _keys_8
        (`MaterialInstanceDynamic.SetScalarParameterValue` (`self.Material Pommel`) (`KismetStringLibrary.Conv_StringToName` _array_element_8) (`BlueprintMapLibrary.Map_Find` (`self.Material1Values`) _array_element_8)))
      (`MaterialInstanceDynamic.SetTextureParameterValue` (`self.Material Pommel`) "M1_Normal" (`self.Pommel M1 - Normal Map`))
      (`MaterialInstanceDynamic.SetTextureParameterValue` (`self.Material Pommel`) "M1_Texture" (`self.Pommel M1 - Texture`))
      (`MaterialInstanceDynamic.SetVectorParameterValue` (`self.Material Pommel`) "M1_Material_Color" (`self.Pommel M1 - Material Color`)))
    (:`then_4`
      ;[1 1 1] Detail
      (bind _output_get_14 (set `self.DetailValues` (`|MakeMap` "Dirt_Contrast" (`self.Dirt Contrast`) "Dirt_Value" (`self.Dirt Value`) "Dirt_Roughness" (`self.Dirt Roughness`) "Damage_Contrast" (`self.Damage Contrast`) "Damage_Value" (`self.Damage Value`) "Blood_Contrast" (`self.Blood Contrast`) "Blood_Value" (`self.Blood Value`) "Blood_Roughness" (`self.Blood Roughness`) "Blood_Metalic" (`self.Blood Metallic`))))
      (bind _keys_9 (`BlueprintMapLibrary.Map_Keys` _output_get_14))
      (for _array_element_9 _keys_9
        (`MaterialInstanceDynamic.SetScalarParameterValue` (`self.Material Pommel`) (`KismetStringLibrary.Conv_StringToName` _array_element_9) (`BlueprintMapLibrary.Map_Find` (`self.DetailValues`) _array_element_9))
        (`MaterialInstanceDynamic.SetScalarParameterValue` (`self.Material Crossguard`) (`KismetStringLibrary.Conv_StringToName` _array_element_9) (`BlueprintMapLibrary.Map_Find` (`self.DetailValues`) _array_element_9))
        (`MaterialInstanceDynamic.SetScalarParameterValue` (`self.Material Blade`) (`KismetStringLibrary.Conv_StringToName` _array_element_9) (`BlueprintMapLibrary.Map_Find` (`self.DetailValues`) _array_element_9))
        (`MaterialInstanceDynamic.SetScalarParameterValue` (`self.Material Grip`) (`KismetStringLibrary.Conv_StringToName` _array_element_9) (`BlueprintMapLibrary.Map_Find` (`self.DetailValues`) _array_element_9)))
      (`MaterialInstanceDynamic.SetVectorParameterValue` (`self.Material Blade`) "Blood_Color" (`self.Blood Color`))
      (`MaterialInstanceDynamic.SetVectorParameterValue` (`self.Material Pommel`) "Blood_Color" (`self.Blood Color`))
      (`MaterialInstanceDynamic.SetVectorParameterValue` (`self.Material Crossguard`) "Blood_Color" (`self.Blood Color`))
      (`MaterialInstanceDynamic.SetVectorParameterValue` (`self.Material Grip`) "Blood_Color" (`self.Blood Color`))
      (`MaterialInstanceDynamic.SetVectorParameterValue` (`self.Material Pommel`) "Dirt_Color" (`self.Dirt Color`))
      (`MaterialInstanceDynamic.SetVectorParameterValue` (`self.Material Blade`) "Dirt_Color" (`self.Dirt Color`))
      (`MaterialInstanceDynamic.SetVectorParameterValue` (`self.Material Crossguard`) "Dirt_Color" (`self.Dirt Color`))
      (`MaterialInstanceDynamic.SetVectorParameterValue` (`self.Material Grip`) "Dirt_Color" (`self.Dirt Color`)))))